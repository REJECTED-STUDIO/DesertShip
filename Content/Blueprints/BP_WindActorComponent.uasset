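; Actor component that pushes a physics-simulated ship with the wind from the level's BP_WindController.
; Each tick it applies delta-scaled force along the wind vector and yaw torque toward the wind heading, both scaled by a sail amount that AddWindScale adjusts and clamps.
; A looping timer on the component itself periodically randomizes the shared controller's wind vector and its own base force scale.
; Ticking is disabled when no controller exists.
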(event Custom|ChangeWind
  (Variables|/Game/Blueprints/BP_WindController.BP_WindController_C|SetWind%20Vector (Variables|Default|GetWind%20Controller) (Math|Vector|MakeVector (Math|Random|RandomFloatinRange -5e+03 5e+03) (Math|Random|RandomFloatinRange -5e+03 5e+03) 0.0))
  (Variables|Default|SetBase%20Wind%20Scale (Math|Random|RandomFloatinRange (Variables|Default|GetMIn%20Base%20Wind%20Scale) (Variables|Default|GetMax%20Base%20Wind%20Scale))))

(event EventBeginPlay
  (Utilities|Time|SetTimerbyEvent (delegate Custom|ChangeWind) 6e+01 true)
  (bind _returnvalue (Actor|GetActorOfClass "/Game/Blueprints/BP_WindController.BP_WindController_C"))
  (Utilities|IsValid _returnvalue
    (:Is%20Valid
      (Variables|Default|SetWind%20Controller _returnvalue)
      (bind _asprimitive_component (Utilities|Casting|CastToPrimitiveComponent (Variables|/Script/Engine.Actor|GetRootComponent (Components|GetOwner))))
      (Variables|Default|SetPrimitive%20Component _asprimitive_component))
    (:Is%20Not%20Valid
      (Components|Tick|SetComponentTickEnabled false))))

(event EventTick
  (params (DeltaSeconds :type Float%20%28single-precision%29))
  (bind _wind_controller (Variables|Default|GetWind%20Controller))
  (bind _primitive_component (Variables|Default|GetPrimitive%20Component))
  (bind _returnvalue (Transformation|GetWorldLocation _primitive_component))
  (bind _returnvalue_2 (Transformation|GetWorldRotation _primitive_component))
  (bind _wind_vector (Variables|/Game/Blueprints/BP_WindController.BP_WindController_C|GetWind%20Vector _wind_controller))
  (bind _returnvalue_3 (+ _returnvalue _wind_vector))
  (bind _returnvalue_4 (Math|Rotator|FindLookatRotation _returnvalue _returnvalue_3))
  (if (> (Variables|Default|GetDynamic%20Wind%20Scale) 0.0)
    (if (Physics|IsSimulatingPhysics (Variables|Default|GetPrimitive%20Component) "None")
      (Physics|AddForce _primitive_component (* _wind_vector (Variables|Default|GetDynamic%20Wind%20Scale) (Variables|Default|GetBase%20Wind%20Scale) (/ 6e+01 (/ 1.0 (Utilities|Time|GetWorldDeltaSeconds)))) "None" false)
      ;[1 1 1] Is facing wind direction
      (if (not (Math|Float|NearlyEqual(Float) (.yaw _returnvalue_2) (.yaw _returnvalue_4) 5.0))
        (Class|PrimitiveComponent|AddTorqueinDegrees (Variables|Default|GetPrimitive%20Component) (Math|Vector|MakeVector 0.0 0.0 (* (Math|Float|SelectFloat -2e+01 2e+01 (> (Class|KismetMathLibrary|FWrap (- (.yaw _returnvalue_2) (.yaw _returnvalue_4)) -1.8e+02 1.8e+02) 0.0)) (Variables|Default|GetDynamic%20Wind%20Scale) (/ 6e+01 (/ 1.0 (Utilities|Time|GetWorldDeltaSeconds))))) "None" true)))))

(fn AddWindScale
  (params (Addition :type Float%20%28double-precision%29))
  (bind _output_get (Variables|Default|SetDynamic%20Wind%20Scale (Math|Float|Clamp(Float) (+ Addition (Variables|Default|GetDynamic%20Wind%20Scale)))))
  ;[1 1 1] Żagiel
  (Development|PrintString (Utilities|String|ToString(Float) _output_get)))