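; BP_WindController is an actor that maintains a wind vector whose direction drifts randomly over time.
; Each Tick rotates WindVector in yaw by a random angle within plus or minus Deviance, scaled by delta time relative to a 60 FPS baseline.
; It then draws a debug arrow from the actor's location along the current wind vector, lasting one tick interval.
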(event EventTick
  (params (DeltaSeconds :type Float%20%28single-precision%29))
  (bind _returnvalue (Transformation|GetActorLocation))
  (bind _deviance (Variables|Default|GetDeviance))
  (Variables|Default|SetWind%20Vector (Math|Vector|RotateVector (Variables|Default|GetWind%20Vector) (Math|Rotator|MakeRotator 0.0 0.0 (* (/ 6e+01 (/ 1.0 DeltaSeconds)) (Math|Random|RandomFloatinRange (* _deviance -1.0) _deviance)))))
  (Rendering|Debug|DrawDebugArrow _returnvalue (+ _returnvalue (Variables|Default|GetWind%20Vector)) 0.0 "(R=0.000000,G=1.000000,B=0.176092,A=1.000000)" (Class|Actor|GetActorTickInterval) 3.0))

(fn ConstructionScript)