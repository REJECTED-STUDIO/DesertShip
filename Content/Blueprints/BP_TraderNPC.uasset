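; Trader NPC that barters: while the shop is open, an actor tagged TradeItem entering the Trade component is destroyed and exchanged for a random item spawned near the NPC.
; Each spawned class is removed from SellItemsPool, which resets to DefaultTradeItems at BeginPlay and on a looping refresh timer.
; OpenShop and CloseShop toggle trading, and debug prints report trade results and list the remaining pool every tick.
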(event OnComponentBeginOverlap(Trade)
  (params (OverlappedComponent :type Primitive%20Component%20Object%20Reference) (OtherActor :type Actor%20Object%20Reference) (OtherComp :type Primitive%20Component%20Object%20Reference) (OtherBodyIndex :type Integer) (bFromSweep :type Boolean) (SweepResult :type Hit%20Result%20Structure%20%28by%20ref%29))
  (if (Variables|Default|GetOpen?)
    (if (Actor|ActorHasTag OtherActor "TradeItem")
      (if (Utilities|Array|IsValidIndex (Variables|Default|GetSellItemsPool) (Math|Random|RandomIntegerinRange 0 -1))
        (Development|PrintString "Sell")
        (Actor|DestroyActor OtherActor)
        (bind _returnvalue (Game|SpawnActorfromClass (Utilities|Array|Get(acopy) (Variables|Default|GetSellItemsPool) (Math|Random|RandomIntegerinRange 0 (Utilities|Array|Length (Variables|Default|GetSellItemsPool)))) (Math|Conversions|ToTransform(Vector) (+ (Transformation|GetWorldLocation (Variables|Default|GetNPC)) "100.000000,-200.000000,200.000000")) "Undefined" "MultiplyWithRoot" 0 0))
        (Utilities|Array|RemoveItem (Variables|Default|GetSellItemsPool) (Utilities|GetClass _returnvalue))
        (else
          (Development|PrintString "Solled All")))
      (else
        (Development|PrintString "No Sell")))
    (else
      (Development|PrintString "Closed"))))

(event Custom|RefreshShop
  (Variables|Default|SetSellItemsPool (Variables|Default|GetDefaultTradeItems))
  (Development|PrintString "Refresh"))

(event Custom|Open%20Shop
  (Variables|Default|SetOpen? true)
  (Development|PrintString "Open Shop" true true "(R=0.000000,G=0.660000,B=1.000000,A=1.000000)" 0.0))

(event Custom|Close%20Shop
  (Variables|Default|SetOpen? false)
  (Development|PrintString "Closed Shop" true true "(R=0.000000,G=0.660000,B=1.000000,A=1.000000)" 0.0))

(event EventTick
  (params (DeltaSeconds :type Float%20%28single-precision%29))
  (for _array_element (Variables|Default|GetSellItemsPool)
    (Development|PrintString (Utilities|GetClassDisplayName _array_element) true true "(R=0.000000,G=0.660000,B=1.000000,A=1.000000)" 0.0)))

(event EventBeginPlay
  (Utilities|Time|SetTimerbyEvent (delegate Custom|RefreshShop) (Variables|Default|GetTimer%20refresh%20Shop) true)
  (Variables|Default|SetSellItemsPool (Variables|Default|GetDefaultTradeItems)))

(fn ConstructionScript)